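; BP_WeaponPickup is a pickup that gives the player a weapon of its item class on use.
; If the player has no weapon, it adds the item, finds an actor of that class in the world via GetActorOfClass, equips it and destroys itself.
; Otherwise it only adds the item and stays in the world, with a free-slot check left as TODO.
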(event EventUse
  (params (Player :type BP%20Player%20Object%20Reference))
  (bind _itemclass (Variables|Default|GetItemClass))
  ;[0 0 0] Called on use. If weapon is equal to null add weapon to inventory and equip it, else add weapon to inventory.
  (if (== (Variables|/Game/Blueprints/Player/BP_Player.BP_Player_C|GetWeapon Player) 0) ; Null check
    (Default|AddItem Player _itemclass)
    (bind _returnvalue (Actor|GetActorOfClass _itemclass)) ; Gets an item of a particular class
    (bind _asbp_weapon (Utilities|Casting|CastToBP_Weapon _returnvalue))
    (Default|EquipWeapon Player _asbp_weapon)
    (Actor|DestroyActor) ; Remove pickup from the world, we don't need it anymore.
    (else
      (Default|AddItem Player (Variables|Default|GetItemClass)) ; TODO: Check for a free weapon slot
    )))

(fn ConstructionScript
  (|CallParentFunction))