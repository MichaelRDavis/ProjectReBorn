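; BP_Pickup is a base pickup actor that shows an item name to the player, with an empty Use function for child Blueprints to override.
; When BP_Player overlaps CollisionComp, it caches the Widget component's Widget_Pickup and sets its name from the first world actor of ItemClass, rather than from itself.
; Any end overlap removes the cached widget from its parent, with no check on the actor.
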(event OnComponentBeginOverlap(CollisionComp)
  (params (OverlappedComponent :type Primitive%20Component%20Object%20Reference) (OtherActor :type Actor%20Object%20Reference) (OtherComp :type Primitive%20Component%20Object%20Reference) (OtherBodyIndex :type Integer) (bFromSweep :type Boolean) (SweepResult :type Hit%20Result%20Structure%20%28by%20ref%29))
  (bind _asbp_player (Utilities|Casting|CastToBP_Player OtherActor))
  (if (Utilities|IsValid _asbp_player)
    (bind _aswidget_pickup (Utilities|Casting|CastToWidget_Pickup (UserInterface|GetUserWidgetObject (Variables|Default|GetWidget))))
    (Variables|Pickup|SetPickupWidget _aswidget_pickup)
    (bind _returnvalue (Actor|GetActorOfClass (Variables|Pickup|GetItemClass)))
    (Variables|/Game/UI/Widget_Pickup.Widget_Pickup_C|SetItemName _aswidget_pickup (Utilities|Text|ToText(String) (Variables|/Game/Blueprints/Actors/BP_InventoryItem.BP_InventoryItem_C|GetItemName _returnvalue)))))

(event OnComponentEndOverlap(CollisionComp)
  (params (OverlappedComponent :type Primitive%20Component%20Object%20Reference) (OtherActor :type Actor%20Object%20Reference) (OtherComp :type Primitive%20Component%20Object%20Reference) (OtherBodyIndex :type Integer))
  (Widget|RemovefromParent (Variables|Pickup|GetPickupWidget)))

(fn ConstructionScript)

(fn Use
  (params (Player :type BP%20Player%20Object%20Reference)))