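; BP_KeyPickup is a usable pickup that gives a key item to the pawn that uses it.
; On BeginPlay it finds an existing actor of ItemClass in the world and, if it is a BP_KeyItem, passes it the pickup's Door reference.
; On use it adds ItemClass to the pawn and destroys itself, or only logs a message if the pawn already holds that item type.
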(event EventOnUsed
  (params (Pawn :type BP%20Player%20Object%20Reference))
  (bind _itemtype (Default|GetItemType Pawn (Variables|Default|GetItemClass)))
  (if (Utilities|IsValid _itemtype)
    (Class|VisualLoggerKismetLibrary|LogText 0 "Key already in inventory" "LogBP_KeyPickup" true)
    (else
      (Default|AddItem Pawn (Variables|Default|GetItemClass))
      (Actor|DestroyActor))))

(event EventBeginPlay
  (bind _returnvalue (Actor|GetActorOfClass (Variables|Default|GetItemClass)))
  (bind _asbp_key_item (Utilities|Casting|CastToBP_KeyItem _returnvalue))
  (Variables|/Game/Blueprints/Actors/BP_KeyItem.BP_KeyItem_C|SetDoor _asbp_key_item (Variables|Default|GetDoor)))

(fn ConstructionScript
  (|CallParentFunction))