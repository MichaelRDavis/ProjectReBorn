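; BP_BaseCharacter is a base character Blueprint that tracks health and handles incoming damage.
; Health starts at MaxHealth on BeginPlay, and positive AnyDamage amounts are subtracted from it.
; Each hit then calls OnDeath when Health reaches zero or below, otherwise OnHit, both of which are empty here.
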(event EventBeginPlay
  (Utilities|FlowControl|Sequence
    (:then_0
      (Variables|Default|SetHealth (Variables|Default|GetMaxHealth)))))

(event Game|Damage|EventAnyDamage
  (params (Damage :type Float%20%28single-precision%29) (DamageType :type Damage%20Type%20Object%20Reference) (InstigatedBy :type Controller%20Object%20Reference) (DamageCauser :type Actor%20Object%20Reference))
  (if (> Damage 0.0)
    (bind _output_get (Variables|Default|SetHealth (- (Variables|Default|GetHealth) Damage)))
    (if (<= _output_get 0.0)
      (CallFunction|OnDeath)
      (else
        (CallFunction|OnHit)))))

(fn ConstructionScript)

(fn OnDeath)

(fn OnHit)