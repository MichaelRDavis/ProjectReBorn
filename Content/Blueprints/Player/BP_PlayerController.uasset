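; Player controller Blueprint that relays movement, sprint and pause input for the player character.
; On BeginPlay it casts the player character to BP_Player and caches it as PlayerOwner.
; Axis events call the character's MoveForward and TurnRight, negating values for backward and left, while Sprint press and release toggle its sprint state.
; PauseGame pauses the game and adds a newly created pause menu widget to the viewport.
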(event EventBeginPlay
  (bind _asbp_player (Utilities|Casting|CastToBP_Player (Game|GetPlayerCharacter 0)))
  (Variables|Default|SetPlayerOwner _asbp_player))

(event Input|ActionEvents|InputActionPauseGame
  (params (Key :type Key%20Structure :default "None"))
  (:Pressed
    (Game|SetGamePaused true)
    (bind _returnvalue (UserInterface|CreateWidget (Variables|Default|GetPauseMenuWIdgetClass) self))
    (UserInterface|Viewport|AddtoViewport _returnvalue 0)))

(event Input|ActionEvents|InputActionSprint
  (params (Key :type Key%20Structure :default "None"))
  (bind _playerowner (Variables|Default|GetPlayerOwner))
  (:Pressed
    (Default|SetIsSprinting _playerowner true)
    (Default|StartSprinting _playerowner))
  (:Released
    (Default|SetIsSprinting _playerowner false)
    (Default|StopSprinting _playerowner)))

(event Input|AxisEvents|InputAxisMoveForward
  (params (AxisValue :type Float%20%28single-precision%29))
  (Default|MoveForward (Variables|Default|GetPlayerOwner) AxisValue))

(event Input|AxisEvents|InputAxisMoveBackward
  (params (AxisValue :type Float%20%28single-precision%29))
  (Default|MoveForward (Variables|Default|GetPlayerOwner) (* AxisValue -1.0)))

(event Input|AxisEvents|InputAxisTurnLeft
  (params (AxisValue :type Float%20%28single-precision%29))
  (Default|TurnRight (Variables|Default|GetPlayerOwner) (* AxisValue -1.0)))

(event Input|AxisEvents|InputAxisTurnRight
  (params (AxisValue :type Float%20%28single-precision%29))
  (Default|TurnRight (Variables|Default|GetPlayerOwner) AxisValue))

(fn ConstructionScript)