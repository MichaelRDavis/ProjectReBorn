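; Player character that handles movement, sprinting, item pickup, inventory and weapon use, viewed through a level BP_CameraActor set as view target on BeginPlay.
; Capsule overlaps track the current BP_UsableActor for Use to trigger.
; Inventory items are spawned actors given to the player, looked up by matching the world's first actor of a class.
; Fire calls forward to the equipped Weapon, while aiming enables its per-tick target lock-on.
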(event OnComponentBeginOverlap(CapsuleComponent)
  (params (OverlappedComponent :type Primitive%20Component%20Object%20Reference) (OtherActor :type Actor%20Object%20Reference) (OtherComp :type Primitive%20Component%20Object%20Reference) (OtherBodyIndex :type Integer) (bFromSweep :type Boolean) (SweepResult :type Hit%20Result%20Structure%20%28by%20ref%29))
  ;[0 0 0] Called on begin overlap
  (if (Utilities|IsValid OtherActor)
    (bind _asbp_usable_actor (Utilities|Casting|CastToBP_UsableActor OtherActor))
    (Variables|Character|SetOverlappedPickup _asbp_usable_actor)
    (bind _output_get (Variables|Character|SetCanPickup true))
    (Class|VisualLoggerKismetLibrary|LogText 0 (Utilities|String|Append "Can Pickup: " (Utilities|String|ToString(Boolean) _output_get)) "LogBP_Player" true)))

(event OnComponentEndOverlap(CapsuleComponent)
  (params (OverlappedComponent :type Primitive%20Component%20Object%20Reference) (OtherActor :type Actor%20Object%20Reference) (OtherComp :type Primitive%20Component%20Object%20Reference) (OtherBodyIndex :type Integer))
  ;[0 0 0] Called on end overlap
  (Variables|Character|SetOverlappedPickup 0)
  (bind _output_get (Variables|Character|SetCanPickup false))
  (Class|VisualLoggerKismetLibrary|LogText 0 (Utilities|String|Append "Can Pickup: " (Utilities|String|ToString(Boolean) _output_get)) "LogBP_Player" true))

(event EventTick
  (params (DeltaSeconds :type Float%20%28single-precision%29))
  (if (Variables|Weapon|GetIsLockedOn)
    (Default|LockonTarget (Variables|Inventory|GetWeapon))))

(event EventBeginPlay
  ;[0 0 0] Initialize player properties
  (|CallParentFunction)
  (bind _returnvalue (Actor|GetActorOfClass "/Game/Blueprints/Actors/BP_CameraActor.BP_CameraActor_C"))
  (Game|Player|SetViewTargetwithBlend (Game|GetPlayerController 0) _returnvalue 0.0 "VTBlend_Linear" 0.0 false))

(fn ConstructionScript
  (|CallParentFunction))

(fn AddItem
  (params (ItemClass :type BP%20Inventory%20Item%20Class%20Reference))
  ;[0 0 0] Add an inventory item to our inventory.
  (bind _returnvalue (Game|SpawnActorfromClass ItemClass (Math|Transform|MakeTransform "0, 0, 0") "AlwaysSpawn" self self))
  (Default|Giveto _returnvalue self) ; We must give ownership of the inventory item to the player.
  (Utilities|Array|AddUnique (Variables|Inventory|GetInventory) _returnvalue))

(fn RemoveItem
  (params (Item :type BP%20Inventory%20Item%20Object%20Reference))
  ;[0 0 0] Remove item from our inventory
  (Default|Remove Item) ; We don't need ownership of it anymore.
  (Utilities|Array|RemoveItem (Variables|Inventory|GetInventory) Item))

(fn DiscardItem
  (params (Item :type BP%20Inventory%20Item%20Object%20Reference))
  (Inventory|RemoveItem Item))

(fn SetIsSprinting
  (params (NewIsSprinting :type Boolean))
  ;[0 0 0] Set sprinting to a new value.
  (Variables|Movement|SetIsSprinting NewIsSprinting))

(fn StartSprinting
  (if (Variables|Movement|GetIsSprinting)
    (Variables|/Script/Engine.CharacterMovementComponent|SetMaxWalkSpeed (Variables|Character|GetCharacterMovement) (Variables|Movement|GetSprintSpeed))))

(fn StopSprinting
  (if (not (Variables|Movement|GetIsSprinting))
    (Variables|/Script/Engine.CharacterMovementComponent|SetMaxWalkSpeed (Variables|Character|GetCharacterMovement) (Variables|Movement|GetDefaultWalkSpeed))))

(fn MoveForward
  (params (Value :type Float%20%28single-precision%29))
  ;[0 0 0] Handles moving forward/backward
  (Pawn|Input|AddMovementInput (Math|Vector|GetForwardVector (Pawn|GetControlRotation :!class /Script/Engine.Pawn)) Value false))

(fn TurnRight
  (params (Value :type Float%20%28single-precision%29))
  ;[0 0 0] Frame rate independent turn
  (Pawn|Input|AddControllerYawInput (* Value (Variables|Movement|GetBaseTurnRate) (Utilities|Time|GetWorldDeltaSeconds))))

(fn GetIsSprinting
  (return (Variables|Movement|GetIsSprinting)))

(fn StartFire
  (bind _weapon (Variables|Inventory|GetWeapon))
  (if (Utilities|IsValid _weapon)
    (Default|StartFire _weapon)))

(fn StopFire
  (bind _weapon (Variables|Inventory|GetWeapon))
  (if (Utilities|IsValid _weapon)
    (Default|StopFire _weapon)))

(fn Use
  (bind _overlappedpickup (Variables|Character|GetOverlappedPickup))
  (if (Utilities|IsValid _overlappedpickup)
    (Default|OnUsed _overlappedpickup self)))

(fn EquipWeapon
  (params (NewWeapon :type BP%20Weapon%20Object%20Reference))
  ;[0 0 0] Equip weapon, sets our current weapon.
  (bind _output_get (Variables|Inventory|SetWeapon NewWeapon))
  (Default|Equip _output_get))

(fn SetIsAiming
  (params (NewIsAiming :type Boolean))
  (Variables|Movement|SetIsAiming NewIsAiming))

(fn GetIsAiming
  (return (Variables|Movement|GetIsAiming)))

(fn StartAiming
  (if (Utilities|IsValid (Variables|Inventory|GetWeapon))
    (Movement|SetIsAiming true)
    (Variables|Weapon|SetIsLockedOn true)))

(fn StopAiming
  (if (Utilities|IsValid (Variables|Inventory|GetWeapon))
    (Movement|SetIsAiming false)
    (Variables|Weapon|SetIsLockedOn false)))

(fn GetItemType
  (params (ItemTypeClass :type BP%20Inventory%20Item%20Class%20Reference))
  (for _array_element (Variables|Inventory|GetInventory)
    (bind _returnvalue (Actor|GetActorOfClass ItemTypeClass))
    (if (== _returnvalue _array_element)
      (return _array_element)
      (else
        (Class|VisualLoggerKismetLibrary|LogText 0 "Item does not exist in inventory" "LogBP_Player" true)))))