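; Weapon blueprint that attaches to its owner's hand socket and fires hitscan shots damaging only BP_Zombie actors.
; StartFire runs a simple state change into FireShot, immediately or after a FireRate timer, though StopFire never reaches EndFiring.
; Each shot line-traces from the owner's eye view, decrements magazine ammo unchecked and plays a sound.
; LockOnTarget sphere-traces around the owner to face a zombie; AddAmmo is an empty stub.
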(event EventBeginPlay
  ;[0 0 0] Initialize weapon properties
  (Utilities|FlowControl|Sequence
    (:then_0
      (if (> (Variables|Weapon|GetMagazineCount) 0)
        (Variables|Weapon|SetMagazineAmmo (Variables|Weapon|GetMaxMagazineAmmo))
        (Variables|Weapon|SetAmmo (* (Variables|Weapon|GetMaxMagazineAmmo) (Variables|Weapon|GetMagazineCount)))))))

(fn ConstructionScript
  (|CallParentFunction))

(fn FireInstantHit
  (bind _itemowner (Variables|Default|GetItemOwner))
  (bind (_outlocation _outrotation) (Actor|GetActorEyesViewPoint _itemowner))
  ;[0 0 0] Fire a line trace from our player view point
  (bind (_outhit _returnvalue) (Collision|LineTraceByChannel _outlocation (+ _outlocation (* (Math|Vector|GetForwardVector _outrotation) (Variables|Weapon|GetWeaponTraceDistance))) "TraceTypeQuery3" true (Utilities|Array|MakeArray self (Variables|Default|GetItemOwner)) "ForDuration" false))
  (if _returnvalue
    (Weapon|ApplyHitDamage _outhit)))

(fn ApplyHitDamage
  (params (HitResult :type Hit%20Result%20Structure))
  (bind (_bblockinghit _binitialoverlap _time _distance _location _impactpoint _normal _impactnormal _physmat _hitactor) (Collision|BreakHitResult HitResult))
  ;[0 0 0] Apply damage on weapon hit
  (bind _asbp_zombie (Utilities|Casting|CastToBP_Zombie _hitactor))
  (Game|Damage|ApplyPointDamage _asbp_zombie (Variables|Weapon|GetHitDamage) _impactpoint HitResult (Game|GetPlayerController 0) self (Variables|Weapon|GetDamageType)))

(fn AttachtoOwner
  (Transformation|AttachComponentToComponent (Variables|Default|GetWeaponMesh) (Variables|/Script/Engine.Character|GetMesh (Variables|Default|GetItemOwner)) (Variables|Weapon|GetHandsAttachSocket) "KeepRelative" "KeepRelative" "KeepRelative" true))

(fn DetachfromOwner
  (Transformation|DetachFromComponent (Variables|Default|GetWeaponMesh) "KeepRelative" "KeepRelative" "KeepRelative" true))

(fn Equip
  (Weapon|AttachtoOwner))

(fn UnEquip
  (Weapon|DetachfromOwner))

(fn GotoState
  (params (NewWeaponState :type EWeaponState%20Enum :default "NewEnumerator0"))
  (LocalVariables|SetPreviousState (Variables|Weapon|GetCurrentWeaponState))
  (if (Utilities|Enum|Equal(Enum) NewWeaponState "NewEnumerator1")
    (Firing|BeginFiring)
    (else
      (Firing|EndFiring))))

(fn StartFire
  (if (not (Variables|Weapon|GetWantsToFire))
    (Variables|Weapon|SetWantsToFire true)
    (Weapon|BeginWeaponState)))

(fn StopFire
  (if (Variables|Weapon|GetWantsToFire)
    (Variables|Weapon|SetWantsToFire false)
    (Weapon|BeginWeaponState)))

(fn Fire
  (Weapon|FireInstantHit))

(fn BeginFiring
  (if (> (Variables|Weapon|GetFireRate) 0.0)
    (bind _returnvalue (Utilities|Time|SetTimerbyFunctionName 0 "FireShot" (Variables|Weapon|GetFireRate)))
    (Variables|Weapon|SetFiringTimer _returnvalue)
    (else
      (Firing|FireShot))))

(fn EndFiring
  (Utilities|Time|ClearandInvalidateTimerbyHandle (Variables|Weapon|GetFiringTimer)))

(fn UseAmmo
  (bind _result (Math|Integer|DecrementInt (Variables|Weapon|GetMagazineAmmo))
    (:%20%20
      (Variables|Weapon|SetMagazineAmmo _result))))

(fn AddAmmo)

(fn FireShot
  (Firing|Fire)
  (Weapon|UseAmmo)
  (Weapon|PlayWeaponFX))

(fn BeginWeaponState
  (if (Variables|Weapon|GetWantsToFire)
    (Weapon|GotoState "NewEnumerator1")))

(fn PlayWeaponFX
  (Audio|PlaySoundatLocation (Variables|Weapon|GetFireSound) (Transformation|GetActorLocation) "0, 0, 0" 1.0 1.0 0.0 0 0 0))

(fn LockonTarget
  (bind _itemowner (Variables|Default|GetItemOwner))
  (bind _returnvalue (Transformation|GetActorLocation _itemowner))
  (bind (_outhit _returnvalue_2) (Collision|SphereTraceByChannel _returnvalue (+ _returnvalue "0, 0,0.100000") (Variables|Weapon|GetLockOnRadius) "TraceTypeQuery2" true (Utilities|Array|MakeArray (Variables|Default|GetItemOwner)) "ForDuration"))
  (if _returnvalue_2
    (bind _asbp_zombie (Utilities|Casting|CastToBP_Zombie (.HitActor (Collision|BreakHitResult _outhit))))
    (Transformation|SetActorRelativeRotation (Variables|Default|GetItemOwner) (Math|Rotator|FindLookatRotation (Transformation|GetActorLocation (Variables|Default|GetItemOwner)) (Transformation|GetActorLocation _asbp_zombie)))))